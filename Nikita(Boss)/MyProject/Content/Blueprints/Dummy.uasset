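; Dummy is an enemy that chases the first player character by calling simple AI move-to-actor every tick.
; On hit, it destroys the other actor unless that actor's class is Dummy.
; Any damage plays the Jump_End animation on its mesh, then destroys the Dummy after a brief delay.
; A delayed branch that would spawn another Dummy at an offset is unwired and never runs.
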(event EventAnyDamage
  (params (Damage :type Float%20%28single-precision%29) (DamageType :type Damage%20Type%20Object%20Reference) (InstigatedBy :type Controller%20Object%20Reference) (DamageCauser :type Actor%20Object%20Reference))
  (Components|Animation|PlayAnimation (Variables|Character|GetMesh) "/Game/Animations/Jump_End.Jump_End" false)
  (Utilities|FlowControl|Delay 0.1)
  (Actor|DestroyActor))

(event EventHit
  (params (MyComp :type Primitive%20Component%20Object%20Reference) (Other :type Actor%20Object%20Reference) (OtherComp :type Primitive%20Component%20Object%20Reference) (bSelfMoved :type Boolean) (HitLocation :type Vector :default "0, 0, 0") (HitNormal :type Vector :default "0, 0, 0") (NormalImpulse :type Vector :default "0, 0, 0") (Hit :type Hit%20Result%20Structure%20%28by%20ref%29))
  (if (!= (Utilities|GetClass Other) "Dummy_C")
    (Actor|DestroyActor Other)))

(event EventTick
  (params (DeltaSeconds :type Float%20%28single-precision%29))
  (AI|Navigation|SimpleMovetoActor (Pawn|GetController) (Game|GetPlayerCharacter 0)))

(fn ConstructionScript)