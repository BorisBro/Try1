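; HealthBox is a health pickup actor that restores a fixed amount of health to the player character and then destroys itself.
; On overlap, it compares the actor's class to player 0's, then heals that player's MyCharacter, clamped to MaxHP, and stays in place if health is full.
; An overlap with any other class, or any hit event, spawns an explosion emitter at the box and destroys it.
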(event EventHit
  (params (MyComp :type Primitive%20Component%20Object%20Reference) (Other :type Actor%20Object%20Reference) (OtherComp :type Primitive%20Component%20Object%20Reference) (bSelfMoved :type Boolean) (HitLocation :type Vector :default "0, 0, 0") (HitNormal :type Vector :default "0, 0, 0") (NormalImpulse :type Vector :default "0, 0, 0") (Hit :type Hit%20Result%20Structure%20%28by%20ref%29))
  ;[1 1 1] SpawnBoxPerTime
  (Effects|SpawnEmitteratLocation "/Game/StarterContent/Particles/P_Explosion.P_Explosion" (Transformation|GetActorLocation))
  (Actor|DestroyActor))

(event EventActorBeginOverlap
  (params (OtherActor :type Actor%20Object%20Reference))
  (bind _returnvalue (Game|GetPlayerCharacter 0))
  ;[1 1 1] SpawnBoxPerTime
  (if (== (Utilities|GetClass OtherActor) (Utilities|GetClass _returnvalue))
    (bind _asmycharacter_c (Utilities|Casting|CastToMyCharacter _returnvalue))
    (if (not (== (Variables|/Game/Blueprints/MyCharacter.MyCharacter_C|Gethealth _asmycharacter_c) (Variables|/Game/Blueprints/MyCharacter.MyCharacter_C|GetMaxHP _asmycharacter_c)))
      (Variables|/Game/Blueprints/MyCharacter.MyCharacter_C|Sethealth _asmycharacter_c (Math|Float|Clamp(Float) (+ (Variables|/Game/Blueprints/MyCharacter.MyCharacter_C|Gethealth _asmycharacter_c) 5e+01) 0.0 (Variables|/Game/Blueprints/MyCharacter.MyCharacter_C|GetMaxHP _asmycharacter_c)))
      (Actor|DestroyActor :!label _label))
    (else
      (Effects|SpawnEmitteratLocation "/Game/StarterContent/Particles/P_Explosion.P_Explosion" (Transformation|GetActorLocation))
      (goto _label))))

(fn ConstructionScript)