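; Dummy is an enemy character that chases the player and deals point damage when it hits an actor of the player's class.
; Tick drives SimpleMoveToActor, jumps at close range and, after a delay when stationary, turns toward the player and leaps using a rotated velocity boost.
; Damage drains its health; at zero it plays an animation, destroys itself and increments MyCharacter's Kills.
; A physics-body spawn on death is left disconnected.
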(event EventHit
  (params (MyComp :type Primitive%20Component%20Object%20Reference) (Other :type Actor%20Object%20Reference) (OtherComp :type Primitive%20Component%20Object%20Reference) (bSelfMoved :type Boolean) (HitLocation :type Vector :default "0, 0, 0") (HitNormal :type Vector :default "0, 0, 0") (NormalImpulse :type Vector :default "0, 0, 0") (Hit :type Hit%20Result%20Structure%20%28by%20ref%29))
  ;[1 1 1] Give Damage
  (if (not (!= (Utilities|GetClass (Game|GetPlayerCharacter 0)) (Utilities|GetClass Other)))
    (Game|Damage|ApplyPointDamage Other 2e+01 HitLocation Hit)))

(event EventAnyDamage
  (params (Damage :type Float%20%28single-precision%29) (DamageType :type Damage%20Type%20Object%20Reference) (InstigatedBy :type Controller%20Object%20Reference) (DamageCauser :type Actor%20Object%20Reference))
  ;[1 1 1] Recieve Damage
  (Variables|Default|SetDummyHealth (- (Variables|Default|GetDummyHealth) Damage))
  (if (not (> (Variables|Default|GetDummyHealth) 0.0))
    (Components|Animation|PlayAnimation (Variables|Character|GetMesh) "/Game/Animations/Jump_End.Jump_End" false)
    (Utilities|FlowControl|Delay 0.2)
    (Actor|DestroyActor)
    (bind _asmycharacter_c (Utilities|Casting|CastToMyCharacter (Game|GetPlayerCharacter 0)))
    (Variables|/Game/Blueprints/MyCharacter.MyCharacter_C|SetKills _asmycharacter_c (+ (Variables|/Game/Blueprints/MyCharacter.MyCharacter_C|GetKills _asmycharacter_c) 1))))

(event EventTick
  (params (DeltaSeconds :type Float%20%28single-precision%29))
  (bind _returnvalue (Transformation|GetActorLocation))
  (bind _returnvalue_2 (Game|GetPlayerCharacter 0))
  (bind _returnvalue_3 (Game|GetPlayerCharacter 0))
  (bind _charactermovement (Variables|Character|GetCharacterMovement))
  (bind _returnvalue_4 (Transformation|GetActorLocation _returnvalue_3))
  (bind _returnvalue_5 (Math|Rotator|FindLookatRotation _returnvalue _returnvalue_4))
  ;[1 1 1] Attack Player
  (Utilities|FlowControl|Sequence
    (:then_0
      (if true
        (Utilities|IsValid _returnvalue_2
          (:Is%20Valid
            (AI|Navigation|SimpleMovetoActor (Pawn|GetController) _returnvalue_2)
            (bind _returnvalue_6 (Transformation|GetDistanceTo _returnvalue_2))
            (Utilities|FlowControl|Sequence
              (:then_0
                (Utilities|FlowControl|Delay 0.5)
                (if (not (!= (Transformation|GetVelocity) "0,0.000000, 0"))
                  (Transformation|SetActorRotation (Class|KismetMathLibrary|MakeRot 0.0 (.Yaw (Class|KismetMathLibrary|BreakRot _returnvalue_5)) 0.0))
                  (Utilities|FlowControl|Delay 0.1)
                  (Character|Jump)
                  (Utilities|FlowControl|Delay 0.25)
                  (Variables|/Script/Engine.MovementComponent|SetVelocity _charactermovement (Math|Vector|RotateVector (+ (Variables|/Script/Engine.MovementComponent|GetVelocity _charactermovement) "500.000000, 0, 0") _returnvalue_5))))
              (:then_1
                (if (< _returnvalue_6 3e+02)
                  (Character|Jump))))))
        (else
          (AI|Navigation|SimpleMovetoActor (Pawn|GetController) self))))))

(fn ConstructionScript)