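; AI dummy character that moves to a destination vector, jumps obstacles and, when its health runs out, plays an animation, destroys itself and increments the player's kills.
; Each tick, forward and downward traces find an obstacle's top, scaling jump velocity to its height and jumping once within range.
; A stuck counter triggers a rotate, jump and velocity push while a move is failing.
; Contact damage logic is disconnected and never runs.
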(event EventHit
  (params (MyComp :type Primitive%20Component%20Object%20Reference) (Other :type Actor%20Object%20Reference) (OtherComp :type Primitive%20Component%20Object%20Reference) (bSelfMoved :type Boolean) (HitLocation :type Vector :default "0, 0, 0") (HitNormal :type Vector :default "0, 0, 0") (NormalImpulse :type Vector :default "0, 0, 0") (Hit :type Hit%20Result%20Structure%20%28by%20ref%29))
  ;[1 1 1] Give Damage
)

(event EventAnyDamage
  (params (Damage :type Float%20%28single-precision%29) (DamageType :type Damage%20Type%20Object%20Reference) (InstigatedBy :type Controller%20Object%20Reference) (DamageCauser :type Actor%20Object%20Reference))
  ;[1 1 1] Recieve Damage
  (Variables|Default|SetDummyHealth (- (Variables|Default|GetDummyHealth) Damage))
  (if (not (> (Variables|Default|GetDummyHealth) 0.0))
    (Components|Animation|PlayAnimation (Variables|Character|GetMesh) "/Game/Animations/Jump_End.Jump_End" false)
    (Utilities|FlowControl|Delay 0.2)
    (Actor|DestroyActor)
    (bind _asmycharacter_c (Utilities|Casting|CastToMyCharacter (Game|GetPlayerCharacter 0)))
    (Variables|/Game/Blueprints/MyCharacter.MyCharacter_C|SetKills _asmycharacter_c (+ (Variables|/Game/Blueprints/MyCharacter.MyCharacter_C|GetKills _asmycharacter_c) 1))))

(event EventTick
  (params (DeltaSeconds :type Float%20%28single-precision%29))
  (bind _returnvalue (Pawn|GetControlRotation :!class /Script/Engine.Pawn))
  (bind _returnvalue_2 (Transformation|GetActorLocation))
  (bind _returnvalue_3 (Transformation|GetActorLocation))
  (bind _returnvalue_4 (* _returnvalue -1.0))
  (bind (_x _y) (Math|Vector|BreakVector _returnvalue_2))
  ;[1 1 1] Jump Func
  (Utilities|FlowControl|Sequence
    (:then_0
      (bind (_outhit _returnvalue_5) (Collision|LineTraceByChannel (+ _returnvalue_3 "0,0.000000,100.000000") (+ (+ (Math|Vector|RotateVector "1000.000000,0.000000,0.000000" (Transformation|GetActorRotation)) _returnvalue_3) "0,0.000000,100.000000") "TraceTypeQuery1" false 0 "None"))
      (if _returnvalue_5
        (bind (_outhit_2 _returnvalue_6) (Collision|LineTraceByChannel (Math|Vector|MakeVector (.X (Math|Vector|BreakVector (.Location (Collision|BreakHitResult _outhit)))) (.Y (Math|Vector|BreakVector (.Location (Collision|BreakHitResult _outhit)))) (+ (.Z (Math|Vector|BreakVector (.Location (Collision|BreakHitResult _outhit)))) 1e+04)) (.Location (Collision|BreakHitResult _outhit)) "TraceTypeQuery1" false 0 "None"))
        (if _returnvalue_6
          (if true
            (Variables|/Script/Engine.CharacterMovementComponent|SetJumpZVelocity (Variables|Character|GetCharacterMovement) (+ (* (Math|Float|Sqrt (.Z (Math|Vector|BreakVector (- (.Location (Collision|BreakHitResult _outhit_2)) (Transformation|GetActorLocation))))) 5e+01) (/ 1e+04 (.Z (Math|Vector|BreakVector (- (.Location (Collision|BreakHitResult _outhit_2)) (Transformation|GetActorLocation)))))))
            (if (< (Math|Float|Absolute(Float) (Math|Float|Sqrt (+ (Math|Float|Power (- (.X (Math|Vector|BreakVector (.Location (Collision|BreakHitResult _outhit_2)))) _x) 2.0) (Math|Float|Power (- (.Y (Math|Vector|BreakVector (.Location (Collision|BreakHitResult _outhit_2)))) _y) 2.0)))) (* (Math|Float|Sqrt (+ (.Z (Math|Vector|BreakVector (- (.Location (Collision|BreakHitResult _outhit_2)) (Transformation|GetActorLocation)))) 5e+01)) 32.0))
              (Utilities|FlowControl|DoOnce false :!label _label
                (:Completed
                  (Character|Jump))))))))
    (:then_1
      (if (== (Variables|/Script/Engine.MovementComponent|GetVelocity (Variables|Character|GetCharacterMovement)) "0, 0, 0")
        (Variables|Default|SetAcceptance%20radius 2e+02)
        (goto _label Reset)))
    (:then_2
      (if (!= (Variables|Default|GetDestinationVector) "0, 0, 0")
        (AI|AIMoveTo self (Variables|Default|GetDestinationVector) 0 (Variables|Default|GetAcceptance%20radius) false
          (:OnSuccess
            (Variables|Default|SetMove? false))
          (:OnFail
            (Variables|Default|SetMove? true)))))
    (:then_3
      (if (== (Variables|/Script/Engine.MovementComponent|GetVelocity (Variables|Character|GetCharacterMovement)) "0, 0, 0")
        (Variables|Default|Setstuck (+ (Variables|Default|Getstuck) 1.0))
        (else
          (Variables|Default|Setstuck 0.0))))
    (:then_4
      (if (and (> (Variables|Default|Getstuck) 5e+01) (Variables|Default|GetMove?))
        (Transformation|SetActorRelativeRotation _returnvalue_4)
        (Utilities|FlowControl|Delay 0.2)
        (Character|Jump)
        (Utilities|FlowControl|Delay 0.2)
        (Variables|/Script/Engine.MovementComponent|SetVelocity (Variables|Character|GetCharacterMovement) (Math|Vector|RotateVector "1000.000000, 0, 0" _returnvalue_4))))))

(event EventOnJumped
  ;[1 1 1] Jump Func
  (Variables|Default|SetAcceptance%20radius 9e+05))

(fn ConstructionScript)