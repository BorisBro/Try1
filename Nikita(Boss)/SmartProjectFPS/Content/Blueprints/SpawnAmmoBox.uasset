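; Spawner actor that places an AmmoBox at its own location and respawns it once the previous one is no longer valid.
; Tick opens a Gate each frame, then closes it while the stored box reference is valid, otherwise runs a Delay before entering the Gate to spawn.
; The delay variable is set to ten seconds after each spawn, so the first spawn uses its default value.
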(event EventTick
  (params (DeltaSeconds :type Float%20%28single-precision%29))
  (Utilities|FlowControl|Sequence
    (:then_0
      (goto _label Open))
    (:then_1
      (Utilities|IsValid (Variables|Default|GetNewVar)
        (:Is%20Valid
          (goto _label Close))
        (:Is%20Not%20Valid
          (Utilities|FlowControl|Delay (Variables|Default|GetDelay))
          (Utilities|FlowControl|Gate true :!label _label
            (:Exit
              (bind _returnvalue (Game|SpawnActorfromClass "/Game/Blueprints/AmmoBox.AmmoBox_C" (Math|Conversions|ToTransform(Vector) (Transformation|GetActorLocation)) false 0))
              (Variables|Default|SetNewVar _returnvalue)
              (Variables|Default|SetDelay 1e+01))))))))

(fn ConstructionScript)