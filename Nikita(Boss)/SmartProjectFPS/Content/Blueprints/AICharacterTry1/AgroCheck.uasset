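; AgroCheck is a behavior tree tick node that detects follow targets around the pawn controlled by Follower_AI_CON.
; Each tick, a sphere trace gathers nearby objects of the desired types, then a Camera-channel line trace checks sight to each.
; A visible hit writes TargetToFollow and TargetLocation to the blackboard, while a blocked one clears TargetToFollow, so the last hit decides.
; Both traces draw debug shapes.
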(event EventTick
  (params (OwnerActor :type Actor%20Object%20Reference) (DeltaSeconds :type Float%20%28single-precision%29))
  (bind _asfollower_ai_con_c (Utilities|Casting|CastToFollower_AI_CON OwnerActor))
  (Variables|Default|SetAI_CON_Ref _asfollower_ai_con_c)
  (Variables|Default|SetMyLocation (Transformation|GetActorLocation (Pawn|GetControlledPawn _asfollower_ai_con_c)))
  (bind _outhits (Collision|MultiSphereTraceForObjects (Transformation|GetActorLocation (Pawn|GetControlledPawn _asfollower_ai_con_c)) (+ (Transformation|GetActorLocation (Pawn|GetControlledPawn _asfollower_ai_con_c)) "0, 0,15.000000") 1.5e+03 (Variables|Default|GetDesiredObjectTypes) false (Utilities|Array|MakeArray (Pawn|GetControlledPawn (Variables|Default|GetAI_CON_Ref))) "ForDuration"))
  (for _array_element _outhits
    (bind _outhit (Collision|LineTraceByChannel (Variables|Default|GetMyLocation) (Transformation|GetActorLocation (.HitActor (Collision|BreakHitResult _array_element))) "TraceTypeQuery2" false (Utilities|Array|MakeArray (Pawn|GetControlledPawn (Variables|Default|GetAI_CON_Ref))) "ForDuration"))
    (if (== (.HitActor (Collision|BreakHitResult _outhit)) (.HitActor (Collision|BreakHitResult _array_element)))
      (Class|BTFunctionLibrary|SetBlackboardValueasObject (Variables|Default|GetTargetToFollow) (.HitActor (Collision|BreakHitResult _outhit)))
      (AI|BehaviorTree|SetBlackboardValueasVector (Variables|Default|GetTargetLocation) (Transformation|GetActorLocation (.HitActor (Collision|BreakHitResult _outhit))))
      (else
        (Class|BTFunctionLibrary|SetBlackboardValueasObject (Variables|Default|GetTargetToFollow))))))