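; ButtonChooseDummy is a world button labeled with a dummy number, apparently for choosing that dummy.
; On BeginPlay it finds its own index among all ButtonChooseDummy actors, stores it as NumberOfDummy and shows a one-based "Dummy" label on its text render.
; Numbering therefore follows GetAllActorsOfClass order rather than a hand-set value.
; Any actor overlap toggles CanPress on begin and end; the press itself is not handled here.
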(event EventActorBeginOverlap
  (params (OtherActor :type Actor%20Object%20Reference))
  (Variables|Default|SetcanPress true))

(event EventActorEndOverlap
  (params (OtherActor :type Actor%20Object%20Reference))
  (Variables|Default|SetcanPress false))

(event EventBeginPlay
  (bind _outactors (Actor|GetAllActorsOfClass "ButtonChooseDummy_C"))
  (for _index (range 0 (Utilities|Array|Length _outactors))
    (if (== (Utilities|Array|Get(acopy) _outactors _index) self)
      (Variables|Default|SetNumberOfDummy _index)
      (Rendering|Components|TextRender|SetText (Variables|Default|GetTextRender1) (Utilities|String|BuildString(Integer) "" "Dummy " (+ _index 1))))))

(fn ConstructionScript)